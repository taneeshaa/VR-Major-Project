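; BP_TV is a television prop for the Classic Mansion that can be switched on or off through IsActive.
; The construction script sets the spotlight intensity and screen material EmissivePower from that flag, adding an audio component only when active.
; On BeginPlay, an active TV plays a timeline that drives the spotlight's intensity over time.
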(event `self.ReceiveBeginPlay`
  (if (`self.IsActive`)
    (bind (_direction _newtrack_0) (`Timeline|Timeline_0`)
      (:`Update`
        (`LightComponent.SetIntensity` (`self.SpotLight`) _newtrack_0)))))

(fn `UserConstructionScript`
  (bind _sm_tv (`self.SM_TV`))
  (bind _spotlight (`self.SpotLight`))
  (if (`self.IsActive`)
    (`LightComponent.SetIntensity` _spotlight 1100.0)
    (`MeshComponent.SetScalarParameterValueOnMaterials` _sm_tv "EmissivePower" 1.0)
    (`AddComponent|NODE_AddAudioComponent-0`)
    (else
      (`LightComponent.SetIntensity` _spotlight 0.0)
      (`MeshComponent.SetScalarParameterValueOnMaterials` _sm_tv "EmissivePower" 0.0))))